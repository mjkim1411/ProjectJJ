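; Rail-shooter player controller that fires the possessed primary character's or drone's gun at the mouse cursor.
; Left click fires once, or in Auto opens a Tick gate that repeats fire, paced by a ShootDelay crosshair flash.
; Shots require ammo, no cinematic, and no crouch or shield.
; Each plays sound, spawns a muzzle projectile, and directly damages the cursor-trace hit, with special effects for SimpleAI1.
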(event `self.ReceiveTick`
  (params (DeltaSeconds :type "Float (single-precision)"))
  (bind _asbp_rail_shoot_game_mode (cast `/Game/BPMain/Interface/Ingame/BP_RailShootGameMode` (`GameplayStatics.GetGameMode`) :!pure true))
  (bind _ashud_cursor (cast `/Game/BPMain/HUD/Interface/HUD_Cursor` (`self.GetHUD`) :!pure true))
  (bind (_bblockinghit _binitialoverlap _time _distance _location _impactpoint _normal _impactnormal _physmat _hitactor) (`GameplayStatics.BreakHitResult` (`self.GetHitResultUnderCursorForObjects` (`|MakeArray` "ObjectTypeQuery1" "ObjectTypeQuery6" :!type "EObjectTypeQuery Enum"))))
  (bind _simpleai_1 (`/Game/BPMain/Interface/Ingame/BP_RailShootGameMode.SimpleAI_1` _asbp_rail_shoot_game_mode))
  (bind _output (`|GetArrayItem` (`/Game/BPMain/Interface/Ingame/BP_RailShootGameMode.PrimaryCH_CPU` _asbp_rail_shoot_game_mode)))
  (bind _output_2 (`|GetArrayItem` (`/Game/BPMain/Interface/Ingame/BP_RailShootGameMode.Drone_CH` _asbp_rail_shoot_game_mode)))
  (bind _returnvalue (`SceneComponent.GetSocketLocation` (`/Game/BPMain/BP_PrimaryCH.M4` (`|GetArrayItem` (`/Game/BPMain/Interface/Ingame/BP_RailShootGameMode.PrimaryCH` _asbp_rail_shoot_game_mode))) "Muzzle"))
  (bind _returnvalue_2 (`SceneComponent.GetSocketLocation` (`/Game/BPMain/BP_Drone_.Ak` _output_2) "Muzzle"))
  (`/Engine/EditorBlueprintResources/StandardMacros.Gate` true :!label _label
    (:`Exit`
      (if (`self.ShootDelay`)
        (set `/Game/BPMain/HUD/Interface/HUD_Cursor.Aim` "/Game/BPMain/Resource/Texture/CrossHairForRailS_Mat_Shoot.CrossHairForRailS_Mat_Shoot" _ashud_cursor)
        (`KismetSystemLibrary.Delay` 0.2)
        (set `/Game/BPMain/HUD/Interface/HUD_Cursor.Aim` "/Game/BPMain/Resource/Texture/CrossHairForRailS_Mat.CrossHairForRailS_Mat" _ashud_cursor)
        (set `self.ShootDelay` false)
        (else
          (if (`/Game/BPMain/Interface/Ingame/BP_RailShootGameMode.CinematicActive` (cast `/Game/BPMain/Interface/Ingame/BP_RailShootGameMode` (`GameplayStatics.GetGameMode`) :!pure true)) :!label _label_2
            _
            (elif (`/Game/BPMain/BP_PrimaryCon.PossessPrimary` _output)
              (if (not (or (`/Game/BPMain/BP_PrimaryCon.CrouchTrue` _output) (== (`/Game/BPMain/BP_PrimaryCon.Ammo` _output) 0)))
                (set `self.ShootDelay` true) ; engage delay for auto mode
                (`/Game/BPMain/BP_PrimaryCon.AmmoUpdate` _output)
                (`GameplayStatics.PlaySoundAtLocation` "/Game/BPMain/Resource/Sound/Gun_SniperRifle_Shot04.Gun_SniperRifle_Shot04" (`self.K2_GetActorLocation` _output) :!label _label_3) ; Play firing sound
                ;[1 1 1] Get Hit Result Under Cursor for Objects (마우스 커서가 가르키는 곳의 물리판정)
                (if (== _hitactor _simpleai_1)
                  ;[1 1 1] SimpleAI1/ Spawn Emitter at location/Visual Effect
                  (if (`/Game/BPMain/ActorClass/SimpleAI.CrouchAnimTrue` _simpleai_1)
                    (`GameplayStatics.SpawnEmitterAtLocation` "/Game/InfinityBladeEffects/Effects/FX_Mobile/Impacts/P_Impact_Shield_Ice.P_Impact_Shield_Ice" _location (struct) (0.5 0.5 0.5))
                    (else
                      (`GameplayStatics.SpawnEmitterAtLocation` "/Game/BPMain/Resource/Particle/P_MuzzleFlash.P_MuzzleFlash" _location (struct) (0.5 0.5 0.5))
                      (bind _returnvalue_3 (`|CreateWidget` "/Game/BPMain/HUD/Combat/ShootEffect.ShootEffect_C"))
                      (`UserWidget.AddToViewport` _returnvalue_3 0))))
                (if (`/Game/BPMain/BP_PrimaryCon.PossessPrimary` _output)
                  (`|SpawnActorFromClass` "/Game/BPMain/ActorClass/BP_ProjectileEnemy.BP_ProjectileEnemy_C" (`KismetMathLibrary.MakeTransform` _returnvalue (`KismetMathLibrary.FindLookAtRotation` _returnvalue _location)) "Undefined" "OverrideRootScale" null null)
                  (else
                    (`|SpawnActorFromClass` "/Game/BPMain/ActorClass/BP_ProjectileEnemy.BP_ProjectileEnemy_C" (`KismetMathLibrary.MakeTransform` _returnvalue_2 (`KismetMathLibrary.FindLookAtRotation` _returnvalue_2 _location)) "Undefined" "OverrideRootScale" null null)))
                (`GameplayStatics.ApplyDamage` _hitactor 50.0))
              (elif (not (or (`/Game/BPMain/BP_Drone_.ShieldOn` _output_2) (== (`/Game/BPMain/BP_Drone_.Ammo` _output_2) 0)))
                (set `self.ShootDelay` true) ; engage delay for auto mode
                (`/Game/BPMain/BP_Drone_.AmmoUpdate` _output_2)
                (goto _label_3)))))))))

(event `Key|LeftMouseButton`
  (params (Key :type "Key Structure"))
  (:`Pressed`
    (if (`self.Auto`)
      (goto _label :!via `Open`)
      (else
        (goto _label_2))))
  (:`Released`
    (goto _label :!via `Close`)))

(fn `UserConstructionScript`)