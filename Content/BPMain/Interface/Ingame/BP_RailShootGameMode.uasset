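; Game mode for a rail-shooter level, handling loading, a countdown timer and area progression.
; BeginPlay shows a loading widget while delayed steps collect both characters and SimpleAI actors and spawn a first enemy, then removes it.
; Once loaded, Tick runs the countdown, pausing at game over, and advances MoveTask on area kills, spawning the next enemy.
; MoveTask indexes locations that auto-move and aim the player's character, while the other character turns toward it.
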(event `self.ReceiveBeginPlay`
  ;[1 1 1] Get All actor of Class /Spawn Actor From class
  (`|ExecutionSequence`
    (:`then_0`
      (bind _returnvalue (`|CreateWidget` "/Game/BPMain/HUD/Interface/LoadingProgress.LoadingProgress_C"))
      (`UserWidget.AddToViewport` _returnvalue 0))
    (:`then_1`
      (`KismetSystemLibrary.Delay` 0.1)
      (bind _outactors (`GameplayStatics.GetAllActorsOfClass` "/Game/BPMain/BP_PrimaryCH.BP_PrimaryCH_C"))
      (set `self.PrimaryCH` _outactors)
      (bind _output_get (set `self.LoadAllActorsNum` (+ (`self.LoadAllActorsNum`) 1) :!label _label))
      (`KismetSystemLibrary.PrintString` (`KismetStringLibrary.Conv_IntToString` _output_get) true true (struct :`R` 1.0 :`B` 0.168745 :`A` 1.0)))
    (:`then_2`
      (`KismetSystemLibrary.Delay` 0.3)
      (bind _outactors_2 (`GameplayStatics.GetAllActorsOfClass` "/Game/BPMain/Dummy/BP_SecondCH.BP_SecondCH_C"))
      (set `self.SecondCH` _outactors_2)
      (goto _label))
    (:`then_3`
      (`KismetSystemLibrary.Delay` 0.5)
      (bind _outactors_3 (`GameplayStatics.GetAllActorsOfClass` "/Game/BPMain/ActorClass/SimpleAI.SimpleAI_C"))
      (set `self.SimpleAI` _outactors_3)
      (goto _label))
    (:`then_4`
      (`KismetSystemLibrary.Delay` 1.0)
      (bind _returnvalue_2 (`|SpawnActorFromClass` "/Game/BPMain/ActorClass/SimpleAI.SimpleAI_C" (`|GetArrayItem` (`self.AISpawnTransF`)) "Undefined" "OverrideRootScale" null null))
      (set `self.SimpleAI_1` _returnvalue_2)
      (goto _label))
    (:`then_10`
      (`KismetSystemLibrary.Delay` 2.0)
      (set `self.IsLoading` false)
      (`Widget.RemoveFromParent` _returnvalue))))

(event `self.ReceiveTick`
  (params (DeltaSeconds :type "Float (single-precision)"))
  (bind _returnvalue (`GameplayStatics.GetPlayerCharacter` 0))
  (bind _move_task (`self.Move_Task`))
  (bind _move_task_2 (`self.Move_Task`))
  (bind _output (`|GetArrayItem` (`self.SecondCH`)))
  (bind _output_2 (`|GetArrayItem` (`self.PrimaryCH`)))
  (if (not (`self.IsLoading`))
    (`|ExecutionSequence`
      (:`then_0`
        ;[1 1 1] 타이머
        (`KismetSystemLibrary.Delay` 1.0)
        (set `self.Seconds` (- (`self.Seconds`) 1))
        (if (< (`self.Seconds`) 0)
          (set `self.Seconds` 59)
          (set `self.Minutes` (- (`self.Minutes`) 1))
          (if (<= (`self.Minutes`) -1)
            (`GameplayStatics.SetGamePaused` true)
            (`KismetSystemLibrary.PrintString` "GaneOver" true true (struct :`R` 1.0 :`B` 0.040439 :`A` 1.0)))))
      (:`then_1`
        ;[1 1 1] SectionReset
        (switch `int` (`self.Move_Task`)
          (:`0`
            (set `self.AreaMaxKill` 1)
            (if (== (`self.Area_Killed`) (`self.AreaMaxKill`))
              (set `self.Move_Task` (+ (`self.Move_Task`) 1))
              (set `self.Area_Killed` 0)
              (`KismetSystemLibrary.PrintString` "Area00" true true (struct :`R` 1.0 :`G` 0.018722 :`A` 1.0))
              (bind _returnvalue_2 (`|SpawnActorFromClass` "/Game/BPMain/ActorClass/SimpleAI.SimpleAI_C" (`|GetArrayItem` (`self.AISpawnTransF`) 1) "Undefined" "OverrideRootScale" null null))
              (set `self.SimpleAI_2` _returnvalue_2)
              (else
                (`KismetSystemLibrary.Delay` 2.0)
                (`KismetSystemLibrary.PrintString` "verse2" true true (struct :`R` 0.813453 :`G` 1.0 :`B` 0.244451 :`A` 1.0)))))
          (:`1`
            (set `self.AreaMaxKill` 1))))
      (:`then_2`
        ;[1 1 1] Player Artificial intelligence
        (`|ExecutionSequence`
          (:`then_0`
            (bind _asbp_primary_ch (cast `/Game/BPMain/BP_PrimaryCH` _returnvalue))
            (bind _returnvalue_3 (`Pawn.GetController` _asbp_primary_ch))
            (`NavigationSystem.SimpleMoveToLocation` _returnvalue_3 (`|GetArrayItem` (`self.Primary_Location`) _move_task_2))
            (`Controller.SetControlRotation` _returnvalue_3 (`KismetMathLibrary.FindLookAtRotation` (`self.K2_GetActorLocation` _asbp_primary_ch) (`|GetArrayItem` (`self.Target_Location`) _move_task_2)))
            (`self.K2_SetActorRotation` _output (`KismetMathLibrary.FindLookAtRotation` (`self.K2_GetActorLocation` _output) (`self.K2_GetActorLocation` _asbp_primary_ch)) false))
          (:`then_1`
            (bind _asbp_second_ch (cast `/Game/BPMain/Dummy/BP_SecondCH` _returnvalue))
            (bind _returnvalue_4 (`Pawn.GetController` _asbp_second_ch))
            (`NavigationSystem.SimpleMoveToLocation` _returnvalue_4 (`|GetArrayItem` (`self.Primary_Location`) _move_task))
            (`Controller.SetControlRotation` _returnvalue_4 (`KismetMathLibrary.FindLookAtRotation` (`self.K2_GetActorLocation` _asbp_second_ch) (`|GetArrayItem` (`self.Target_Location`) _move_task)))
            (`self.K2_SetActorRotation` _output_2 (`KismetMathLibrary.FindLookAtRotation` (`self.K2_GetActorLocation` _output_2) (`self.K2_GetActorLocation` _asbp_second_ch)) false)))
        (switch `int` _move_task)))))

(fn `UserConstructionScript`)