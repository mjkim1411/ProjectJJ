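; BP_PrimaryCon is the primary player pawn in a rail shooter, showing its HUD while possessed and holding ammo, armor and health.
; LeftCtrl both crouches and reloads from reserve ammo, with a sound and timed reload flag.
; CharaterSwap, outside cinematics, spawns and possesses a CharacterSawpper at the camera to switch to character two.
; Damage functions ignore their input: TakeDamege decrements armor, then health, while TakeDamageForAI subtracts zero.
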(event `self.ReceivePossessed`
  (params (NewController :type "Controller Object Reference"))
  (bind _returnvalue (`|CreateWidget` "/Game/BPMain/HUD/Ability/RSHUD_Primary.RSHUD_Primary_C"))
  (`UserWidget.AddToViewport` _returnvalue 0))

(event `self.ReceiveUnpossessed`
  (params (OldController :type "Controller Object Reference"))
  ;[1 1 1] Remove Hud
  (`WidgetLayoutLibrary.RemoveAllWidgets`))

(event `Key|LeftControl`
  (params (Key :type "Key Structure"))
  ;[1 1 1] Crouch/Reloading
  (:`Pressed`
    (bind (_output_get _output_get1 _output_get2) (`self.Reload`))
    (set `self.CrouchTrue` true)
    (if (or _output_get _output_get1 _output_get2)
      (`GameplayStatics.SpawnSoundAtLocation` "/Game/BPMain/Resource/Sound/Reload.Reload" (`self.K2_GetActorLocation`))
      (`KismetSystemLibrary.Delay` 2.8)
      (set `self.IsReloading` false)))
  (:`Released`
    (set `self.CrouchTrue` false)))

(event `InputAction|CharaterSwap`
  (params (Key :type "Key Structure"))
  (bind _primarycam (`self.PrimaryCam`))
  (:`Pressed`
    ;[1 1 1] 캐릭터 스왑(구)
    (if (not (`/Game/BPMain/Interface/Ingame/BP_RailShootGameMode.CinematicActive` (cast `/Game/BPMain/Interface/Ingame/BP_RailShootGameMode` (`GameplayStatics.GetGameMode`) :!pure true)))
      (bind _returnvalue (`|SpawnActorFromClass` "/Game/BPMain/Interface/Ingame/CharacterSawpper.CharacterSawpper_C" (`KismetMathLibrary.MakeTransform` (`SceneComponent.K2_GetComponentLocation` _primarycam) (`SceneComponent.K2_GetComponentRotation` _primarycam)) "Undefined" "OverrideRootScale" null null))
      (`Controller.Possess` (`self.GetController` (`GameplayStatics.GetPlayerPawn` 0)) _returnvalue)
      (message `/Game/BPMain/Interface/Ingame/ActionInterFace.CharaterSwapping` _returnvalue _primarycam true))))

(fn `AmmoUpdate`
  (set `self.Ammo` (- (`self.Ammo`) 1)))

(fn `Reload`
  (returns (Output_Get :type Boolean) (Output_Get1 :type Boolean) (Output_Get2 :type Boolean))
  (bind _returnvalue (- (`self.ClipSize`) (`self.Ammo`)))
  ;[1 1 1] Conversation Ammo
  (if (< (`self.Ammo`) (`self.ClipSize`))
    (if (> (`self.MaxAmmo`) _returnvalue)
      (set `self.AmmoDefference` _returnvalue)
      (set `self.Ammo` (+ (`self.Ammo`) (`self.AmmoDefference`)))
      (set `self.MaxAmmo` (- (`self.MaxAmmo`) (`self.AmmoDefference`)))
      (bind _output_get (set `self.IsReloading` true))
      (return _output_get (stale _output_get_3) (stale _output_get_2))
      (elif (< (`self.MaxAmmo`) 1)
        (bind _output_get_2 (set `self.IsReloading` false))
        (else
          (set `self.AmmoDefference` _returnvalue)
          (set `self.Ammo` (+ (`self.Ammo`) (`self.MaxAmmo`)))
          (set `self.MaxAmmo` 0)
          (bind _output_get_3 (set `self.IsReloading` true)))))
    (else
      (`KismetSystemLibrary.PrintString` "Full Ammo"))))

(fn `TakeDamageForAI`
  (params (Damage :type "Float (double-precision)"))
  (set `self.Health` (- (`self.Health`) (* 0.0 0.0))))

(fn `TakeDamege`
  (params (Damage :type "Float (double-precision)"))
  (bind _output_get (set `self.Armor` (- (`self.Armor`) 1.0)))
  (if (< _output_get 0.0)
    (set `self.Health` (- (`self.Health`) 1.0))))

(fn `UserConstructionScript`)