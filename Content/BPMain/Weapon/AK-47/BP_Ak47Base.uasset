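; AK-47 base weapon Blueprint that tracks clip and reserve ammo for the player's rifle.
; Reload tops up the clip from MaxAmmo, sets IsReloading on the player's BP_PrimaryCH according to available reserve, and prints a notice when full.
; Fire is an empty event; its projectile, ammo-use and muzzle flash logic is disconnected, as is an alternative reload that discards leftover rounds.
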(event `Fire`)

(fn `Reload`
  (returns (Output_Get :type Boolean) (Output_Get1 :type Boolean) (Output_Get2 :type Boolean))
  (bind _returnvalue (- (`self.ClipSize`) (`self.Ammo`)))
  (bind _asbp_primary_ch (cast `/Game/BPMain/BP_PrimaryCH` (`GameplayStatics.GetPlayerCharacter` 0) :!pure true))
  ;[1 1 1] Conversation Ammo
  (if (< (`self.Ammo`) (`self.ClipSize`))
    (if (> (`self.MaxAmmo`) _returnvalue)
      (set `self.AmmoDefference` _returnvalue)
      (set `self.Ammo` (+ (`self.Ammo`) (`self.AmmoDefference`)))
      (set `self.MaxAmmo` (- (`self.MaxAmmo`) (`self.AmmoDefference`)))
      (bind _output_get (set `/Game/BPMain/BP_PrimaryCH.IsReloading` true (cast `/Game/BPMain/BP_PrimaryCH` (`GameplayStatics.GetPlayerCharacter` 0) :!pure true)))
      (return _output_get (stale _output_get_3) (stale _output_get_2))
      (elif (< (`self.MaxAmmo`) 1)
        (bind _output_get_2 (set `/Game/BPMain/BP_PrimaryCH.IsReloading` false _asbp_primary_ch))
        (else
          (set `self.AmmoDefference` _returnvalue)
          (set `self.Ammo` (+ (`self.Ammo`) (`self.MaxAmmo`)))
          (set `self.MaxAmmo` 0)
          (bind _output_get_3 (set `/Game/BPMain/BP_PrimaryCH.IsReloading` true _asbp_primary_ch)))))
    (else
      (`KismetSystemLibrary.PrintString` "Full Ammo"))))

(fn `UserConstructionScript`)