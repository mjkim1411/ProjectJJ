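; M4A1 weapon base Blueprint with a Fire event that is currently empty, so this graph adds no firing behavior.
; An unwired chain holds projectile spawning at the Muzzle socket, ammo decrement and a scaled-down muzzle flash on the player's equipped weapon.
; A second unwired chain repeats only the flash, casting the player to BP_PrimaryCH and reading the weapon's SkeletalMesh socket.
; The construction script is empty.
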(event `Fire`)

(fn `UserConstructionScript`)