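; Low-range enemy AI pawn that roams, spots the player and dies from accumulated damage.
; Tick issues delayed random nav-point moves until PawnSensing sets CanSeePlayer, which is never cleared; non-lethal hits before that trigger a short random move.
; Sighting runs DoOnce-gated chained AIMoveTo calls toward player character classes, with no attack logic.
; At zero Health, IsDead disables movement, then after a delay the actor is destroyed and a KillPickUp widget appears.
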(event `self.ReceiveAnyDamage`
  (params (Damage :type "Float (single-precision)") (DamageType :type "DamageType Object Reference") (InstigatedBy :type "Controller Object Reference") (DamageCauser :type "Actor Object Reference"))
  ;[1 1 1] 피격에 대한 것
  (bind _output_get (set `self.Health` (- (`self.Health`) Damage)))
  (if (<= _output_get 0.0)
    (set `self.IsDead` true)
    (`KismetSystemLibrary.Delay` 5.0)
    (`self.K2_DestroyActor`)
    (bind _returnvalue (`|CreateWidget` "/Game/BPMain/HUD/Combat/KillPickUp.KillPickUp_C"))
    (`UserWidget.AddToViewport` _returnvalue 0)
    (cast `/Game/BPMain/Interface/Ingame/ProtoMapGameState` (`GameplayStatics.GetGameState`))
    (else
      ;[1 1 1] Smart AI (피격후 Chase) 이동
      (if (not (`self.CanSeePlayer`))
        (`|AIMoveTo` self (`NavigationSystem.K2_GetRandomLocationInNavigableRadius` (`self.K2_GetActorLocation`) 250.0))))))

(event `FacePlayer`
  ;[1 1 1] FacePlayer
  (`self.K2_SetActorRotation` (`GameplayStatics.GetPlayerCharacter` 0) (`KismetMathLibrary.FindLookAtRotation` (`self.K2_GetActorLocation`) (`self.K2_GetActorLocation` (`GameplayStatics.GetPlayerCharacter` 0))) false))

(event `self.PawnSensing.OnSeePawn`
  (params (Pawn :type "Pawn Object Reference"))
  ;[1 1 1] Chase and Attack
  (`/Engine/EditorBlueprintResources/StandardMacros.DoOnce` false :!label _label
    (:`Completed`
      (cast `/Game/BPMain/Dummy/BP_FirstPersonChar` Pawn)
      (set `self.CanSeePlayer` true)
      (`KismetSystemLibrary.PrintString` "Can not See player I'm LowRangeEnemy")
      (`|AIMoveTo` self (0.0 0.0 0.0) null 300.0
        (:`OnSuccess`
          _)
        (:`OnFail`
          _))
      (`|AIMoveTo` self (0.0 0.0 0.0) (cast `/Game/BPMain/Dummy/BP_FirstPersonSecondChar` Pawn :!pure true) 300.0
        (:`OnSuccess`
          (goto _label :!via `Reset`))
        (:`OnFail`
          (goto _label :!via `Reset`))))))

(event `self.ReceiveTick`
  (params (DeltaSeconds :type "Float (single-precision)"))
  ;[1 1 1] AI Roaming
  (`|ExecutionSequence`
    (:`then_0`
      (`KismetSystemLibrary.Delay` 3.0)
      (if (not (`self.CanSeePlayer`))
        (`|AIMoveTo` self (`NavigationSystem.K2_GetRandomLocationInNavigableRadius` (`self.K2_GetActorLocation`) 600.0))))
    (:`then_1`
      ;[1 1 1] IsDeadState
      (if (`self.IsDead`)
        (`CharacterMovementComponent.DisableMovement` (`self.CharacterMovement`))))))

(fn `UserConstructionScript`)