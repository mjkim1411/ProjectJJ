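; Primary character Blueprint for a rail shooter, handling damage reactions for both possessed and unpossessed states.
; AnyDamage routes damage to the game mode's first PrimaryCHCPU entry and ignores it while crouched.
; When possessed, remaining armor shows cracked glass; depleted armor shows a vignette, then after a delay resets armor and rebuilds the HUD.
; When unpossessed, it applies AI damage and spawns blood at the SimpleAI attacker's bullet point.
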(event `self.ReceiveAnyDamage`
  (params (Damage :type "Float (single-precision)") (DamageType :type "DamageType Object Reference") (InstigatedBy :type "Controller Object Reference") (DamageCauser :type "Actor Object Reference"))
  (bind _output (`|GetArrayItem` (`/Game/BPMain/Interface/Ingame/BP_RailShootGameMode.PrimaryCH_CPU` (cast `/Game/BPMain/Interface/Ingame/BP_RailShootGameMode` (`GameplayStatics.GetGameMode`) :!pure true))))
  (bind _crouchtrue (`/Game/BPMain/BP_PrimaryCon.CrouchTrue` _output))
  ;[1 1 1] Anydamage
  (if (`/Game/BPMain/BP_PrimaryCon.PossessPrimary` _output)
    (if (not _crouchtrue)
      (`/Game/BPMain/BP_PrimaryCon.TakeDamege` _output Damage)
      (if (>= (`/Game/BPMain/BP_PrimaryCon.Armor` _output) 0.0)
        (bind _returnvalue (`|CreateWidget` "/Game/BPMain/HUD/Combat/GlassCrack_Pre.GlassCrack_Pre_C"))
        (`UserWidget.AddToViewport` _returnvalue 0)
        (else
          (bind _returnvalue_2 (`|CreateWidget` "/Game/BPMain/HUD/Combat/DamageVignette.DamageVignette_C"))
          (`UserWidget.AddToViewport` _returnvalue_2 0)
          (`KismetSystemLibrary.Delay` 2.0)
          (`WidgetLayoutLibrary.RemoveAllWidgets`)
          (set `/Game/BPMain/BP_PrimaryCon.Armor` 3.0 _output)
          (bind _returnvalue_3 (`|CreateWidget` "/Game/BPMain/HUD/Ability/RSHUD_Primary.RSHUD_Primary_C"))
          (`UserWidget.AddToViewport` _returnvalue_3 0))))
    (elif (not _crouchtrue)
      (`/Game/BPMain/BP_PrimaryCon.TakeDamageForAI` _output Damage)
      (bind _assimple_ai (cast `/Game/BPMain/ActorClass/SimpleAI` DamageCauser))
      (bind _returnvalue_4 (`GameplayStatics.SpawnEmitterAtLocation` "/Game/BPMain/Resource/Particle/P_blood.P_blood" (`/Game/BPMain/ActorClass/SimpleAI.BulletPointForAi` _assimple_ai)))
      (`SceneComponent.SetWorldScale3D` _returnvalue_4 (0.5 0.5 0.5)))))

(fn `UserConstructionScript`)