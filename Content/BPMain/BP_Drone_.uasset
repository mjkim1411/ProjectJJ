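; Player drone for a rail shooter that can hand control over to another character through the CharaterSwap input.
; Unless the game mode flags an active cinematic, the input spawns a CharacterSawpper at the drone camera's transform and possesses it.
; The swapper then receives the camera and a flag marking the switch as not toward character 2.
; A separate AmmoUpdate function decrements the drone's Ammo by one.
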(event `InputAction|CharaterSwap`
  (params (Key :type "Key Structure"))
  (bind _camera (`self.Camera`))
  ;[1 1 1] 캐릭터 스왑(신)
  (:`Pressed`
    ;[1 1 1] 캐릭터 스왑(구)
    (if (not (`/Game/BPMain/Interface/Ingame/BP_RailShootGameMode.CinematicActive` (cast `/Game/BPMain/Interface/Ingame/BP_RailShootGameMode` (`GameplayStatics.GetGameMode`) :!pure true)))
      (bind _returnvalue (`|SpawnActorFromClass` "/Game/BPMain/Interface/Ingame/CharacterSawpper.CharacterSawpper_C" (`KismetMathLibrary.MakeTransform` (`SceneComponent.K2_GetComponentLocation` _camera) (`SceneComponent.K2_GetComponentRotation` _camera)) "Undefined" "OverrideRootScale" null null))
      (`Controller.Possess` (`self.GetController` (`GameplayStatics.GetPlayerPawn` 0)) _returnvalue)
      (message `/Game/BPMain/Interface/Ingame/ActionInterFace.CharaterSwapping` _returnvalue _camera false))))

(fn `AmmoUpdate`
  (set `self.Ammo` (- (`self.Ammo`) 1)))

(fn `UserConstructionScript`)