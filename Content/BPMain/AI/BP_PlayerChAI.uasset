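; AI controller for the player character in a rail shooter, handing its control to a behavior tree.
; On BeginPlay it prints a debug string, initializes BB_PrimaryCPU, copies MoveTask from BP_RailShootGameMode into the blackboard, then runs BT_PrimaryCPU.
; An unconnected AIMoveTo toward the game mode's SecondLocation entry indexed by MoveTask never runs.
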(event `self.ReceiveBeginPlay`
  ;[1 1 1] Behevior
  (`KismetSystemLibrary.PrintString` "PrimaryCPU)RUn")
  (`self.UseBlackboard` "/Game/BPMain/AI/PrimaryAI/BB_PrimaryCPU.BB_PrimaryCPU")
  (`BlackboardComponent.SetValueAsInt` (`AIBlueprintHelperLibrary.GetBlackboard` self) (`self.MoveTask`) (`/Game/BPMain/Interface/Ingame/BP_RailShootGameMode.Move_Task` (cast `/Game/BPMain/Interface/Ingame/BP_RailShootGameMode` (`GameplayStatics.GetGameMode`) :!pure true)))
  (`self.RunBehaviorTree` "/Game/BPMain/AI/PrimaryAI/BT_PrimaryCPU.BT_PrimaryCPU"))

(fn `UserConstructionScript`)